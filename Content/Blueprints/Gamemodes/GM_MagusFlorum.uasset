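; Game mode for Magus Florum that runs the level flow, tracks collectibles and respawns the player.
; A state machine broadcasts each change through a dispatcher, starting music at setup, showing an end-of-level widget and loading the next level.
; Killed events from player and cat pawns respawn the same class at the active checkpoint or PlayerStart, then possess it.
; The win check tests CatsNeeded for zero, separately from the collected counters.
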(event `self.ReceiveTick`
  (params (DeltaSeconds :type "Float (single-precision)"))
  ;[1 0.3731 0] Debugging
  (bind (_current_hours _current_minutes _current_seconds _time_as_string) (`self.Get time in game`))
  (`KismetSystemLibrary.PrintString` (`KismetStringLibrary.Concat_StrStr` "Current game state: " (`|GetEnumeratorNameAsString` (`self.Game state`)) " \nCats needed: " (`KismetStringLibrary.Conv_IntToString` (`self.Cats needed`)) " \nCats collected: " (`KismetStringLibrary.Conv_IntToString` (`self.Cats collected`)) " \nTime in game: " _time_as_string) true true (struct :`G` 0.66 :`B` 1.0 :`A` 1.0) DeltaSeconds))

(event `self.ReceiveBeginPlay`
  ;[1 1 1] Init
  (`self.Change game state` "NewEnumerator0")
  (`self.Bind player instance`))

(event `Bind player instance`
  ;[1 1 1] Get reference to player
  (bind _asbp_player_pawn (cast `/Game/Blueprints/Actors/Characters/BP_PlayerPawn` (`GameplayStatics.GetPlayerCharacter` 0)))
  (set `self.Player ref` _asbp_player_pawn) ; Update player ref to\nnew player instance
  (add `/Game/Blueprints/Actors/Characters/BP_PlayerPawn.ED_PlayerKilled` (`self.Player ref`) (`|CreateDelegate` :!event `Player killed`)) ; Bind player character killed event
  (bind _returnvalue (`GameplayStatics.GetActorOfClass` "/Game/Blueprints/Actors/Characters/BP_CatPawn.BP_CatPawn_C"))
  (`/Engine/EditorBlueprintResources/StandardMacros.IsValid` _returnvalue
    (:`Is Valid`
      (add `/Game/Blueprints/Actors/Characters/BP_CatPawn.ED_PlayerKilled` _returnvalue (`|CreateDelegate` :!event `Player killed`)) ; Bind cat character killed event
    )))

(event `Change game state`
  (params (`New state` :type "/Game/Blueprints/Data/E_GameStates Enum" :default "NewEnumerator0"))
  ;[1 1 1] Change current game state
  (bind _output_get (set `self.Game state` `New state`))
  (`KismetSystemLibrary.PrintString` (`KismetStringLibrary.Concat_StrStr` "Gamestate change: " (`|GetEnumeratorNameAsString` _output_get)) true true (struct :`R` 1.0 :`G` 0.373139 :`A` 1.0))
  (`self.GameStateChange` _output_get) ; Trigger event dispatcher to notify other\nblueprints of the new state
  (switch `/Game/Blueprints/Data/E_GameStates` _output_get
    (:`NewEnumerator0`
      (`self.Setup`))
    (:`NewEnumerator1`
      (`self.Game start`))
    (:`NewEnumerator2`
      (`self.In game`))
    (:`NewEnumerator3`
      (`self.End game`))
    (:`NewEnumerator4`
      (`self.Post game`))))

(event `Setup`
  ;[1 1 1] Game states
  (set `self.Cats in level` (`self.Cats needed`))
  (`self.Change game state` "NewEnumerator1")
  (bind _returnvalue (`GameplayStatics.CreateSound2D` "/Game/Assets/Audio/Cues/SC_MainMenuMusic.SC_MainMenuMusic" 1.0 1.0 0.0 null))
  (bind _output_get (set `self.Music ref` _returnvalue))
  (`AudioComponent.Play` _output_get 0.0))

(event `Game start`
  ;[1 1 1] Game states
  (`self.Change game state` "NewEnumerator2"))

(event `In game`
  ;[1 1 1] Game states
)

(event `End game`
  ;[1 1 1] Game states
  (bind _returnvalue (`|CreateWidget` "/Game/UI/UI_EndOfLevel.UI_EndOfLevel_C"))
  (`UserWidget.AddToViewport` _returnvalue 0))

(event `Post game`
  ;[1 1 1] Game states
  (bind _asgi_game_instance (cast `/Game/Blueprints/GI_GameInstance` (`GameplayStatics.GetGameInstance`)))
  (`/Game/Blueprints/GI_GameInstance.Load next level` _asgi_game_instance))

(event `Check win condition`
  ;[1 1 1] Win condition
  (`self.CheckWinCondition`
    (:`true`
      (`self.Change game state` "NewEnumerator3"))))

(event `Update game stats`
  (params (`Item collected` :type "/Game/Blueprints/Data/E_Collectables Enum" :default "NewEnumerator0"))
  ;[1 1 1] Update game stats
  (switch `/Game/Blueprints/Data/E_Collectables` `Item collected`
    (:`NewEnumerator1`
      (`/Engine/EditorBlueprintResources/StandardMacros.IncrementInt` (`self.Cats collected`)
        (:`  `
          (`KismetSystemLibrary.PrintString` "Cat collected!" true true (struct :`R` 0.056174 :`G` 1.0 :`A` 1.0)))))
    (:`NewEnumerator0`
      (`/Engine/EditorBlueprintResources/StandardMacros.IncrementInt` (`self.Coins collected`)
        (:`  `
          (`KismetSystemLibrary.PrintString` "Coin collected!" true true (struct :`R` 0.056174 :`G` 1.0 :`A` 1.0)))))
    (:`NewEnumerator2`
      (`/Engine/EditorBlueprintResources/StandardMacros.IncrementInt` (`self.Yarn collected`)
        (:`  `
          (`KismetSystemLibrary.PrintString` "Yarn collected!" true true (struct :`R` 0.056174 :`G` 1.0 :`A` 1.0)))))))

(event `SetActiveCheckpoint`
  (params (Checkpoint :type "/Game/Blueprints/Actors/BP_Checkpoint Object Reference"))
  ;[1 1 1] Set active checkpoint
  (set `self.Active checkpoint` Checkpoint)
  (`KismetSystemLibrary.PrintString` "Checkpoint set!" true true (struct :`R` 0.056174 :`G` 1.0 :`A` 1.0)))

(event `Player killed`
  (params (`Character ref` :type "Character Object Reference"))
  (bind _spawn_transform (`self.Spawn transform`))
  ;[1 1 1] Respawn chracter
  (set `self.Character to re-spawn` (`GameplayStatics.GetObjectClass` `Character ref`)) ; Who was the player controlling\nwhen they were killed?
  (`KismetSystemLibrary.Delay` 2.0)
  (if (`KismetSystemLibrary.IsValid` (`self.Active checkpoint`))
    (set `self.Spawn transform` (`self.GetTransform` (`self.Active checkpoint`))) ; Set spawn transform to that \nof the active checkpoint actor
    (else
      (bind _returnvalue (`GameplayStatics.GetActorOfClass` "/Script/Engine.PlayerStart")) ; Find player start actor
      (set `self.Spawn transform` (`self.GetTransform` _returnvalue)) ; Set spawn transform to that \nof the player start actor
    ))
  (bind _returnvalue_2 (`|SpawnActorFromClass` (`self.Character to re-spawn`) (`KismetMathLibrary.MakeTransform` (`KismetMathLibrary.TransformLocation` _spawn_transform) (`KismetMathLibrary.TransformRotation` _spawn_transform)) "AdjustIfPossibleButAlwaysSpawn" "OverrideRootScale" null null)) ; Spawn new player character at the spawn transform
  (`Controller.Possess` (`GameplayStatics.GetPlayerController` 0) _returnvalue_2) ; Possess the new player character
  (`self.Bind player instance`)
  (`KismetSystemLibrary.PrintString` "Player re-spawned!" true true (struct :`R` 0.056174 :`G` 1.0 :`A` 1.0)))

(fn `Get time in game`
  (returns (`Current hours` :type Integer) (`Current minutes` :type Integer) (`Current seconds` :type Integer) (`Time as string` :type String))
  (locals (Hours :type Integer :default 0) (Minutes :type Integer :default 0) (Seconds :type Integer :default 0) (`Hours string` :type String) (`Minutes string` :type String) (`Seconds string` :type String))
  (bind _returnvalue (`KismetStringLibrary.Conv_IntToString` (`local.Hours`)))
  (bind _returnvalue_2 (`KismetStringLibrary.Conv_IntToString` (`local.Minutes`)))
  (bind _returnvalue_3 (`KismetStringLibrary.Conv_IntToString` (`local.Seconds`)))
  (bind (_returnvalue_days _returnvalue_hours _returnvalue_minutes _returnvalue_seconds) (`KismetMathLibrary.BreakTimespan` (`KismetMathLibrary.MakeTimespan` 0 0 0 (`KismetMathLibrary.FTrunc` (`GameplayStatics.GetRealTimeSeconds`)))))
  (set `local.Hours` _returnvalue_hours)
  (set `local.Minutes` _returnvalue_minutes)
  (set `local.Seconds` _returnvalue_seconds)
  (`|ExecutionSequence`
    (:`then_0`
      ;[1 1 1] Add leading zeros?
      (if (< (`local.Hours`) 10)
        (set `local.Hours string` (`KismetStringLibrary.Concat_StrStr` "0" _returnvalue))
        (else
          (set `local.Hours string` _returnvalue))))
    (:`then_1`
      (if (< (`local.Minutes`) 10)
        (set `local.Minutes string` (`KismetStringLibrary.Concat_StrStr` "0" _returnvalue_2))
        (else
          (set `local.Minutes string` _returnvalue_2))))
    (:`then_2`
      (if (< (`local.Seconds`) 10)
        (set `local.Seconds string` (`KismetStringLibrary.Concat_StrStr` "0" _returnvalue_3))
        (else
          (set `local.Seconds string` _returnvalue_3))))
    (:`then_3`
      ;[1 1 1] Output
      (return (`local.Hours`) (`local.Minutes`) (`local.Seconds`) (`KismetStringLibrary.Concat_StrStr` (`local.Hours string`) ":" (`local.Minutes string`) ":" (`local.Seconds string`))))))

(fn `UserConstructionScript`)