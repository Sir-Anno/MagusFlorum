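; Timed effect component that makes the player pawn invulnerable for a set duration, set on BeginPlay before calling the parent effect logic.
; EffectStart casts the owner to BP_PlayerPawn and disables damage on its health component, and EffectEnd re-enables it.
; Start, per-second tick and end events each call the parent and print colored debug messages to the screen.
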(event `self.ReceiveBeginPlay`
  (set `self.Effect duration` 10)
  (`parent.ReceiveBeginPlay`))

(event `self.Effect start`
  (`parent.Effect start`)
  (`KismetSystemLibrary.PrintString` "Player  invulnerability in effect" true true (struct :`R` 0.056174 :`G` 1.0 :`A` 1.0) 0.5)
  (bind _asbp_player_pawn (cast `/Game/Blueprints/Actors/Characters/BP_PlayerPawn` (`self.GetOwner`)))
  (set `/Game/Blueprints/Components/C_HealthComponent.CanTakeDamage?` false (`/Game/Blueprints/Actors/Characters/BP_PlayerPawn.C_HealthComponent` _asbp_player_pawn)))

(event `self.Effect tick`
  (`parent.Effect tick`)
  (`KismetSystemLibrary.PrintString` "Player is invulnerability" true true (struct :`R` 1.0 :`G` 0.73919 :`A` 1.0) 0.5))

(event `self.Effect end`
  (`parent.Effect end`)
  (`KismetSystemLibrary.PrintString` "Player  invulnerability has ended" true true (struct :`R` 1.0 :`G` 0.007198 :`A` 1.0) 0.5)
  (bind _asbp_player_pawn (cast `/Game/Blueprints/Actors/Characters/BP_PlayerPawn` (`self.GetOwner`)))
  (set `/Game/Blueprints/Components/C_HealthComponent.CanTakeDamage?` true (`/Game/Blueprints/Actors/Characters/BP_PlayerPawn.C_HealthComponent` _asbp_player_pawn)))