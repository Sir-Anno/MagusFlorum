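; Health component that tracks damage and healing for its owning actor and can destroy that actor.
; BeginPlay caches the owner; the damage event subtracts Health, then runs a CheckDeath macro whose Killed output destroys the owner.
; As wired, CheckDeath exits Alive at zero or below and Killed otherwise.
; Separate TakeDamage and AddHealth functions sit beside the events, the latter empty.
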(event `self.ReceiveBeginPlay`
  ;[1 1 1] Set reference of what actor the component is attached to
  (set `self.OwnedActor` (`self.GetOwner`)))

(event `Take damage`
  (params (Damage :type "Float (double-precision)"))
  ;[1 1 1] Take damage event
  (set `self.Health` (- (`self.Health`) Damage))
  (`self.CheckDeath?`
    (:`Killed`
      (`Actor.K2_DestroyActor` (`self.OwnedActor`)))))

(event `Add health`
  (params (Health :type "Float (double-precision)"))
  ;[1 1 1] Add health event
  (set `self.Health` (+ (`self.Health`) Health)))

(fn `AddHealth`
  (params (Health :type "Float (double-precision)")))

(fn `TakeDamage`
  (params (Damage :type "Float (double-precision)"))
  (set `self.Health` (- (`self.Health`) Damage)))