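; A timed effect component that changes the mana of the BP_PlayerPawn that owns it.
; BeginPlay sets the effect duration before calling the parent class, which handles the effect lifecycle, and EffectStart caches the owning pawn.
; Each EffectTick, noted as once per second, adds ManaChangeAmount through the pawn's mana component.
; Start, tick and end each print a colored debug message.
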(event `self.ReceiveBeginPlay`
  (set `self.Effect duration` 10) ; This is handled by the parent class
  (`parent.ReceiveBeginPlay`))

(event `self.Effect start`
  (`parent.Effect start`)
  (`KismetSystemLibrary.PrintString` "Mana modifier in effect" true true (struct :`R` 0.056174 :`G` 1.0 :`A` 1.0) 0.5)
  (bind _asbp_player_pawn (cast `/Game/Blueprints/Actors/Characters/BP_PlayerPawn` (`self.GetOwner`)))
  (set `self.Player ref` _asbp_player_pawn))

(event `self.Effect tick`
  (`parent.Effect tick`)
  (`KismetSystemLibrary.PrintString` "Mana is being modified" true true (struct :`R` 1.0 :`G` 0.73919 :`A` 1.0) 0.5)
  (`/Game/Blueprints/Components/C_ManaComponent.Add mana` (`/Game/Blueprints/Actors/Characters/BP_PlayerPawn.C_ManaComponent` (`self.Player ref`)) (`self.ManaChangeAmount`)))

(event `self.Effect end`
  (`parent.Effect end`)
  (`KismetSystemLibrary.PrintString` "Mana modifier  has ended" true true (struct :`R` 1.0 :`G` 0.007198 :`A` 1.0) 0.5))