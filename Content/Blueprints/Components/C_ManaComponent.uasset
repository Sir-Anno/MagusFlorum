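; Actor component that manages a mana pool for its owning actor, which it caches on BeginPlay.
; UseMana deducts a cost only when the availability check finds enough mana.
; AddMana and RemoveMana change the value and broadcast it with the owner through the EDManaChange dispatcher.
; AddMana clamps only the broadcast value to MaxMana, not the stored Mana, and RemoveMana does not clamp.
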(event `self.ReceiveBeginPlay`
  ;[1 1 1] Set reference of what actor the component is attached to
  (set `self.OwnedActor` (`self.GetOwner`)))

(event `Use mana`
  (params (`Mana cost` :type Integer))
  (`self.CheckManaAvaliable?` `Mana cost`
    (:`Can cast`
      (`self.Remove mana` `Mana cost`))))

(event `Add mana`
  (params (Amount :type Integer))
  (bind _output_get (set `self.Mana` (+ (`self.Mana`) Amount)))
  (`self.ED_ManaChange` (`KismetMathLibrary.Clamp` _output_get 0 (`self.Max mana`)) (`self.OwnedActor`)))

(event `Remove mana`
  (params (Amount :type Integer))
  (bind _output_get (set `self.Mana` (- (`self.Mana`) Amount)))
  (`self.ED_ManaChange` _output_get (`self.OwnedActor`)))