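; Effect component that modifies the owning player pawn's health over time, built on a parent effect class that drives its start, tick and end events.
; BeginPlay sets the effect duration before calling the parent.
; Each tick, fired every second, casts the owner to BP_PlayerPawn and adds HealthAmount through its health component.
; Start, tick and end also print colored debug messages.
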(event `self.ReceiveBeginPlay`
  (set `self.Effect duration` 10) ; This is handled by the parent class
  (`parent.ReceiveBeginPlay`))

(event `self.Effect start`
  (`KismetSystemLibrary.PrintString` "Health modifier in effect" true true (struct :`R` 0.056174 :`G` 1.0 :`A` 1.0) 0.5))

(event `self.Effect tick`
  (`KismetSystemLibrary.PrintString` "Health is being modified" true true (struct :`R` 1.0 :`G` 0.73919 :`A` 1.0) 0.5)
  (bind _asbp_player_pawn (cast `/Game/Blueprints/Actors/Characters/BP_PlayerPawn` (`self.GetOwner`)))
  (`/Game/Blueprints/Components/C_HealthComponent.Add health` (`/Game/Blueprints/Actors/Characters/BP_PlayerPawn.C_HealthComponent` _asbp_player_pawn) (`self.Health amount`)))

(event `self.Effect end`
  (`KismetSystemLibrary.PrintString` "Health modifier has ended" true true (struct :`R` 1.0 :`G` 0.007198 :`A` 1.0) 0.5))