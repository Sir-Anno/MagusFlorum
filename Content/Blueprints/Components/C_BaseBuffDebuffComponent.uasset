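; Base component for timed buff and debuff effects on the player pawn, with start, tick and end events for child effect components.
; On BeginPlay it adds itself to the player's HUD and starts the effect, doing nothing if the owner is not BP_PlayerPawn.
; A looping one-second timer ticks the effect and decrements its duration, then clears itself and ends the effect.
; Each event's base implementation calls a matching event dispatcher.
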(event `self.ReceiveBeginPlay`
  (bind _output_get (set `self.Attached actor` (`self.GetOwner`)))
  (bind _asbp_player_pawn (cast `/Game/Blueprints/Actors/Characters/BP_PlayerPawn` _output_get))
  (`/Game/UI/UI_HUD.Effect added` (`/Game/Blueprints/Actors/Characters/BP_PlayerPawn.HUD UI Ref` _asbp_player_pawn) self) ; Notify UI of new effect \nto add icon to screen
  (`self.Effect start`)
  (bind _returnvalue (`KismetSystemLibrary.K2_SetTimerDelegate` (delegate `Tick`) 1.0 true))
  (set `self.Timer` _returnvalue))

(event `Tick`
  (if (> (`self.Effect duration`) 0)
    (`self.Effect tick`)
    (`/Engine/EditorBlueprintResources/StandardMacros.DecrementInt` (`self.Effect duration`))
    (else
      (`KismetSystemLibrary.K2_ClearAndInvalidateTimerHandle` (`self.Timer`))
      (`self.Effect end`))))

(event `Effect start`
  ;[1 1 1] Used by child effect components
  (`self.ED_EffectStart`))

(event `Effect tick`
  ;[1 1 1] Used by child effect components
  (`self.ED_EffectTick`))

(event `Effect end`
  ;[1 1 1] Used by child effect components
  (`self.ED_EffectEnd`))