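; Timed effect component that temporarily scales the player pawn's walk speed by a multiplier.
; It sets a ten-second duration and relies on its parent class for the start, per-second tick and end events.
; On start it caches BP_PlayerPawn's MaxWalkSpeed and applies SpeedMultiplier, then on end restores the cached speed and destroys itself.
; Each stage prints a colored on-screen status message.
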(event `self.ReceiveBeginPlay`
  (set `self.Effect duration` 10) ; This is handled by the parent class
  (`parent.ReceiveBeginPlay`))

(event `self.Effect start`
  (`parent.Effect start`)
  (`KismetSystemLibrary.PrintString` "Player speed has changed" true true (struct :`R` 0.056174 :`G` 1.0 :`A` 1.0) 0.5)
  ;[1 1 1] Get the player character movement component
  (bind _asbp_player_pawn (cast `/Game/Blueprints/Actors/Characters/BP_PlayerPawn` (`self.GetOwner`)))
  (bind _output_get (set `self.Character Movement` (`Character.CharacterMovement` _asbp_player_pawn)))
  ;[1 1 1] Remember default movement speed
  (set `self.DefaultWalkSpeed` (`CharacterMovementComponent.MaxWalkSpeed` _output_get))
  ;[1 1 1] Set movement speed boost
  (set `CharacterMovementComponent.MaxWalkSpeed` (* (`self.DefaultWalkSpeed`) (`self.SpeedMultiplier`)) (`self.Character Movement`)))

(event `self.Effect tick`
  (`parent.Effect tick`)
  (`KismetSystemLibrary.PrintString` "Player speed is being altered" true true (struct :`R` 1.0 :`G` 0.73919 :`A` 1.0) 0.5))

(event `self.Effect end`
  (`parent.Effect end`)
  (`KismetSystemLibrary.PrintString` "Player speed has reset" true true (struct :`R` 1.0 :`G` 0.007198 :`A` 1.0) 0.5)
  (set `CharacterMovementComponent.MaxWalkSpeed` (`self.DefaultWalkSpeed`) (`self.Character Movement`))
  (`self.K2_DestroyComponent`))