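; Timed mana regeneration effect component that restores the player's mana over a fixed duration.
; BeginPlay sets the effect duration, then defers to the parent class, which handles the effect lifecycle.
; Each one-second tick casts the owner to BP_PlayerPawn and adds ManaRegen through its mana component.
; Start, tick and end events print short color-coded debug messages.
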(event `self.ReceiveBeginPlay`
  (set `self.Effect duration` 10) ; This is handled by the parent class
  (`parent.ReceiveBeginPlay`))

(event `self.Effect start`
  (`KismetSystemLibrary.PrintString` "Effect started" true true (struct :`R` 0.056174 :`G` 1.0 :`A` 1.0) 0.5))

(event `self.Effect tick`
  (`KismetSystemLibrary.PrintString` "Effect tick" true true (struct :`R` 1.0 :`G` 0.73919 :`A` 1.0) 0.5)
  (bind _asbp_player_pawn (cast `/Game/Blueprints/Actors/Characters/BP_PlayerPawn` (`self.GetOwner`)))
  (`/Game/Blueprints/Components/C_ManaComponent.Add mana` (`/Game/Blueprints/Actors/Characters/BP_PlayerPawn.C_ManaComponent` _asbp_player_pawn) (`self.ManaRegen`)))

(event `self.Effect end`
  (`KismetSystemLibrary.PrintString` "Effect ended" true true (struct :`R` 1.0 :`G` 0.007198 :`A` 1.0) 0.5))