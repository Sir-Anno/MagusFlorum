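; Casting component for the player pawn that spawns a BP_Rose where the camera trace lands when E is pressed while aiming.
; It caches its owner on BeginPlay and casts it to BP_PlayerPawn to read the aiming flag.
; A Visibility line trace from the camera, offset by its rotation scaled by TraceDistance, supplies the spawn location, with debug drawing on and no check for a hit.
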(event `self.ReceiveBeginPlay`
  ;[1 1 1] Set reference of what actor the component is attached to
  (set `self.OwnedActor` (`self.GetOwner`)))

(event `Key|E`
  (params (Key :type "Key Structure"))
  (bind _returnvalue (`GameplayStatics.GetPlayerCameraManager` 0))
  (bind _returnvalue_2 (`PlayerCameraManager.GetCameraLocation` _returnvalue))
  ;[1 1 1] Spawn rose
  (:`Pressed`
    (bind _asbp_player_pawn (cast `/Game/Blueprints/Actors/Characters/BP_PlayerPawn` (`self.OwnedActor`)))
    (if (`/Game/Blueprints/Actors/Characters/BP_PlayerPawn.IsAming?` _asbp_player_pawn)
      (bind _outhit (`KismetSystemLibrary.LineTraceSingle` _returnvalue_2 (+ _returnvalue_2 (* (`PlayerCameraManager.GetCameraRotation` _returnvalue) (`self.Trace distance`))) "TraceTypeQuery1" false (`|MakeArray` (`GameplayStatics.GetPlayerCharacter` 0) :!type "Actor Object Reference") "ForDuration" true (struct :`R` 1.0 :`A` 1.0) (struct :`G` 1.0 :`A` 1.0) 1.0))
      (`|SpawnActorFromClass` "/Game/Blueprints/Actors/BP_Rose.BP_Rose_C" (`KismetMathLibrary.Conv_VectorToTransform` (`.Location` (`GameplayStatics.BreakHitResult` _outhit))) "Undefined" "OverrideRootScale" null null))))