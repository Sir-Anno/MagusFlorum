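; C_SpeedModifier is a timed effect component that scales the walk speed of its owning BP_PlayerPawn by SpeedMultiplier.
; It sets the effect duration before calling the parent BeginPlay, which handles timing, and implements the start, tick and end events.
; Start multiplies MaxWalkSpeed after a brief delay, while end resets it to a hard-coded default rather than the previous value and destroys the component.
; Tick only prints debug text.
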(event `self.ReceiveBeginPlay`
  (set `self.Effect duration` 10) ; This is handled by the parent class
  (`parent.ReceiveBeginPlay`))

(event `self.Effect start`
  (bind _speedmultiplier (`self.SpeedMultiplier`))
  (`KismetSystemLibrary.PrintString` "Effect started" true true (struct :`R` 0.056174 :`G` 1.0 :`A` 1.0) 0.5)
  (`KismetSystemLibrary.Delay` 0.01)
  (bind _asbp_player_pawn (cast `/Game/Blueprints/Actors/Characters/BP_PlayerPawn` (`self.GetOwner`)))
  (bind _output_get (set `self.Character Movement` (`Character.CharacterMovement` _asbp_player_pawn)))
  (`KismetSystemLibrary.PrintString` (`KismetStringLibrary.Conv_DoubleToString` _speedmultiplier))
  (set `CharacterMovementComponent.MaxWalkSpeed` (* (`CharacterMovementComponent.MaxWalkSpeed` _output_get) _speedmultiplier) _output_get))

(event `self.Effect tick`
  (`KismetSystemLibrary.PrintString` "Effect tick" true true (struct :`R` 1.0 :`G` 0.73919 :`A` 1.0) 0.5))

(event `self.Effect end`
  (`KismetSystemLibrary.PrintString` "Effect ended" true true (struct :`R` 1.0 :`G` 0.007198 :`A` 1.0) 0.5)
  (set `CharacterMovementComponent.MaxWalkSpeed` 500.0 (`self.Character Movement`))
  (`self.K2_DestroyComponent`))