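; C_CastingSpeedModifier is a timed effect component that temporarily scales the player's casting speed.
; It sets a fixed effect duration on BeginPlay, then defers to its parent class, whose start, tick and end events it extends.
; On start it caches the owning BP_PlayerPawn's casting speed and applies a multiplier to the casting component.
; On end it restores the cached value; the tick only calls the parent.
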(event `self.ReceiveBeginPlay`
  (set `self.Effect duration` 10) ; This is handled by the parent class
  (`parent.ReceiveBeginPlay`))

(event `self.Effect start`
  (`parent.Effect start`)
  ;[1 1 1] Get the default casting speed from the casting component
  (bind _asbp_player_pawn (cast `/Game/Blueprints/Actors/Characters/BP_PlayerPawn` (`self.GetOwner`)))
  (bind _output_get (set `self.Player ref` _asbp_player_pawn))
  (bind _output_get_2 (set `self.Default casting speed` (`/Game/Blueprints/Components/C_CastingComponent.Casting speed` (`/Game/Blueprints/Actors/Characters/BP_PlayerPawn.C_CastingComponent` _output_get))))
  ;[1 1 1] Modify the casting speed
  (set `/Game/Blueprints/Components/C_CastingComponent.Casting speed` (* _output_get_2 (`self.Casting Speed multiplyer`)) (`/Game/Blueprints/Actors/Characters/BP_PlayerPawn.C_CastingComponent` (`self.Player ref`))))

(event `self.Effect tick`
  (`parent.Effect tick`))

(event `self.Effect end`
  (`parent.Effect end`)
  ;[1 1 1] Reset the casting speed
  (set `/Game/Blueprints/Components/C_CastingComponent.Casting speed` (`self.Default casting speed`) (`/Game/Blueprints/Actors/Characters/BP_PlayerPawn.C_CastingComponent` (`self.Player ref`))))