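; Actor component that lets its owner carry and place a crystal in the crystal network.
; On BeginPlay it spawns a BP_PickedUpCrystal in front of the owner, and each Tick keeps it ahead of the owner at a lowered height.
; Interact, gated by a DoOnce that resets shortly after spawn, replaces the carried crystal with a BP_MovableCrystal at its location, then destroys the component.
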(event `self.ReceiveBeginPlay`
  (bind _returnvalue (`self.GetOwner`))
  (`KismetSystemLibrary.PrintString` "PickedUpCrystal")
  (bind _returnvalue_2 (`|SpawnActorFromClass` "/Game/Blueprints/Actors/CrystalNetwork/BP_PickedUpCrystal.BP_PickedUpCrystal_C" (`KismetMathLibrary.MakeTransform` (+ (* (`Actor.GetActorForwardVector` _returnvalue) 80.0) (`Actor.K2_GetActorLocation` _returnvalue))) "Undefined" "OverrideRootScale" null null))
  (set `self.Crystal` _returnvalue_2)
  (`KismetSystemLibrary.Delay` 0.2)
  (`self.Reset`))

(event `self.ReceiveTick`
  (params (DeltaSeconds :type "Float (single-precision)"))
  (bind _returnvalue (`self.GetOwner`))
  (bind _crystal (`self.Crystal`))
  (bind (_returnvalue_x _returnvalue_y _returnvalue_z) (`KismetMathLibrary.BreakVector` (+ (* (`Actor.GetActorForwardVector` _returnvalue) 150.0) (`Actor.K2_GetActorLocation` _returnvalue))))
  (`/Engine/EditorBlueprintResources/StandardMacros.IsValid` _crystal
    (:`Is Valid`
      (`Actor.K2_SetActorLocation` _crystal (`KismetMathLibrary.MakeVector` _returnvalue_x _returnvalue_y (- _returnvalue_z 95.0)) false false))))

(event `/Game/Blueprints/Interfaces/BI_Interact.Interact`
  (params (Player :type "Character Object Reference"))
  (bind _returnvalue (`Actor.K2_GetActorLocation` (`self.Crystal`)))
  (`KismetSystemLibrary.PrintString` "Interacted")
  (`/Engine/EditorBlueprintResources/StandardMacros.DoOnce` true :!label _label
    (:`Completed`
      (set `self.CrystalLocation` _returnvalue)
      (`|SpawnActorFromClass` "/Game/Blueprints/Actors/CrystalNetwork/BP_MovableCrystal.BP_MovableCrystal_C" (`KismetMathLibrary.MakeTransform` _returnvalue) "Undefined" "OverrideRootScale" null null)
      (`Actor.K2_DestroyActor` (`self.Crystal`))
      (`KismetSystemLibrary.PrintString` "Place Crystal")
      (`self.K2_DestroyComponent`))))

(event `Reset`
  (goto _label :!via `Reset`))