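; Interactable spawner actor that creates a BP_Boulder at its SpawnPosition, allowing only one live boulder at a time.
; Interacting while it is available spawns the boulder with a back-reference to the spawner and calls ReverseGrow on every entry in Leaves.
; UpdateSpawnerState derives availability from the boulder reference and swaps the Cube material to show it.
; RemoveSpawnedBoulderRef clears that reference to re-enable spawning.
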(event `self.ReceiveBeginPlay`
  (`self.UpdateSpawnerState`))

(event `/Game/Blueprints/Interfaces/BI_Interact.Interact`
  (params (Player :type "Character Object Reference"))
  (if (`self.CanSpawnBoulder`)
    (`self.SpawnBoulder`)
    (`self.ResetLeaves`)))

(event `SpawnBoulder`
  (bind _returnvalue (`|SpawnActorFromClass` "/Game/Blueprints/Actors/BoulderActors/BP_Boulder.BP_Boulder_C" (`KismetMathLibrary.MakeTransform` (.location (`SceneComponent.K2_GetComponentToWorld` (`self.SpawnPosition`))) (.rotation (`SceneComponent.K2_GetComponentToWorld` (`self.SpawnPosition`)))) "Undefined" "OverrideRootScale" null self null))
  (set `self.SpawnedBoulder` _returnvalue)
  (`self.UpdateSpawnerState`))

(event `ResetLeaves`
  (for _array_element (`self.Leaves`)
    (`/Game/Blueprints/Actors/BoulderActors/BP_Leaf.ReverseGrow` _array_element)))

(fn `RemoveSpawnedBoulderRef`
  (set `self.SpawnedBoulder` null)
  (`self.UpdateSpawnerState`))

(fn `UpdateSpawnerState`
  (bind _returnvalue (not (`KismetSystemLibrary.IsValid` (`self.SpawnedBoulder`))))
  (set `self.CanSpawnBoulder` _returnvalue)
  (`PrimitiveComponent.SetMaterial` (`self.Cube`) 0 (select `bool` _returnvalue :`false` (`self.CanNotSpawnMaterial`) :`true` (`self.CanSpawnMaterial`) :!type "MaterialInterface Object Reference")))

(fn `UserConstructionScript`)