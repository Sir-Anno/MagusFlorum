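; BP_Leaf is an interactable leaf actor that grows and retracts, toggling whether it blocks.
; Interact triggers Grow, which plays the growth animation on the skeletal mesh and makes the Box collision block all channels.
; ReverseGrow plays the reverse animation and sets the Box to ignore collision, with a leftover debug print.
; A HasGrown flag guards both, and an option can disable collision at BeginPlay.
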(event `self.ReceiveBeginPlay`
  (if (`self.DisableCollisionOnBeginPlay`)
    (`PrimitiveComponent.SetCollisionResponseToAllChannels` (`self.Box`) "ECR_Ignore")))

(event `/Game/Blueprints/Interfaces/BI_Interact.Interact`
  (params (Player :type "/Game/Blueprints/Actors/Characters/BP_PlayerPawn Object Reference"))
  (`self.Grow`))

(event `Grow`
  (if (not (`self.HasGrown`))
    (set `self.HasGrown` true)
    (`SkeletalMeshComponent.PlayAnimation` (`self.SkeletalMesh`) "/Game/Assets/Animations/Leaf/Leaf_Anim_Growth.Leaf_Anim_Growth" false)
    (`PrimitiveComponent.SetCollisionResponseToAllChannels` (`self.Box`) "ECR_Block")))

(event `ReverseGrow`
  (`KismetSystemLibrary.PrintString` "Hello")
  (if (`self.HasGrown`)
    (set `self.HasGrown` false)
    (`SkeletalMeshComponent.PlayAnimation` (`self.SkeletalMesh`) "/Game/Assets/Animations/Leaf/Leaf_Anim_Reverse.Leaf_Anim_Reverse" false)
    (`PrimitiveComponent.SetCollisionResponseToAllChannels` (`self.Box`) "ECR_Ignore")))

(fn `UserConstructionScript`)