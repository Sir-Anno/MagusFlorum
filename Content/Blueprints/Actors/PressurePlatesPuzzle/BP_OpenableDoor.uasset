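; An actor door for a pressure plate puzzle that opens when all of its linked plates are active at once.
; On BeginPlay it binds to the activate and deactivate events of player, plant and cat plate arrays, counting the total.
; Those events adjust an active count; matching the total plays a timeline that lerps the door to its end location.
; Deactivating a plate only lowers the count and does not close the door.
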(event `self.ReceiveBeginPlay`
  (for _array_element (`self.PlayerPressurePlates`)
    (add `/Game/Blueprints/Actors/PressurePlatesPuzzle/BP_PlayerPressurePlate.E_PlateActivated` _array_element (`|CreateDelegate` :!event `PressurePlateActive`))
    (add `/Game/Blueprints/Actors/PressurePlatesPuzzle/BP_PlayerPressurePlate.E_PlateDeactivated` _array_element (`|CreateDelegate` :!event `PressurePlateDeactive`))
    (`/Engine/EditorBlueprintResources/StandardMacros.IncrementInt` (`self.TotalPlates`)))
  (for _array_element_2 (`self.PlantPressurePlates`)
    (add `/Game/Blueprints/Actors/PressurePlatesPuzzle/BP_PlantPressurePlate.E_PlantPlateActivated` _array_element_2 (`|CreateDelegate` :!event `PressurePlateActive`))
    (add `/Game/Blueprints/Actors/PressurePlatesPuzzle/BP_PlantPressurePlate.E_PlantPlateDeactivated` _array_element_2 (`|CreateDelegate` :!event `PressurePlateDeactive`))
    (`/Engine/EditorBlueprintResources/StandardMacros.IncrementInt` (`self.TotalPlates`)))
  (for _array_element_3 (`self.CatPressurePlates`)
    (add `/Game/Blueprints/Actors/PressurePlatesPuzzle/BP_CatPressurePlate.E_CatPlateActivated` _array_element_3 (`|CreateDelegate` :!event `PressurePlateActive`))
    (add `/Game/Blueprints/Actors/PressurePlatesPuzzle/BP_CatPressurePlate.E_CatPlateDeactivated` _array_element_3 (`|CreateDelegate` :!event `PressurePlateDeactive`))
    (`/Engine/EditorBlueprintResources/StandardMacros.IncrementInt` (`self.TotalPlates`))))

(event `PressurePlateActive`
  (bind _result (`/Engine/EditorBlueprintResources/StandardMacros.IncrementInt` (`self.ActivePlates`))
    (:`  `
      (if (== _result (`self.TotalPlates`))
        (`self.OpenDoor`)))))

(event `PressurePlateDeactive`
  (`/Engine/EditorBlueprintResources/StandardMacros.DecrementInt` (`self.ActivePlates`)))

(event `OpenDoor`
  (set `self.StartLocation` (`self.K2_GetActorLocation`))
  (bind (_direction _opendoor) (`Timeline|T_OpenDoor`)
    (:`Update`
      (`self.K2_SetActorLocation` (`KismetMathLibrary.VLerp` (`self.StartLocation`) (`self.EndLocation`) _opendoor)))))

(fn `UserConstructionScript`)