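; Test interactable actor that logs player proximity and grants a child effect component when interacted with.
; A range sphere, sized from InteractRange in the construction script, prints colored debug messages as BP_PlayerPawn enters or leaves it.
; The Interact event prints a message, then adds the template-named C_ChildEffectComponentDUPLICATETHIS to the player pawn found through player index 0, without checking range itself.
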(event `self.InteractRangeSphere.OnComponentBeginOverlap`
  (params (OverlappedComponent :type "PrimitiveComponent Object Reference") (OtherActor :type "Actor Object Reference") (OtherComp :type "PrimitiveComponent Object Reference") (OtherBodyIndex :type Integer) (bFromSweep :type Boolean) (SweepResult :type "HitResult Structure (by ref)"))
  (cast `/Game/Blueprints/Actors/Characters/BP_PlayerPawn` OtherActor)
  (`KismetSystemLibrary.PrintString` "Player entered interact range" true true (struct :`R` 0.056174 :`G` 1.0 :`A` 1.0)))

(event `self.InteractRangeSphere.OnComponentEndOverlap`
  (params (OverlappedComponent :type "PrimitiveComponent Object Reference") (OtherActor :type "Actor Object Reference") (OtherComp :type "PrimitiveComponent Object Reference") (OtherBodyIndex :type Integer))
  (cast `/Game/Blueprints/Actors/Characters/BP_PlayerPawn` OtherActor)
  (`KismetSystemLibrary.PrintString` "Player left interact range" true true (struct :`R` 1.0 :`G` 0.007198 :`A` 1.0)))

(event `/Game/Blueprints/Interfaces/BI_Interact.Interact`
  (`KismetSystemLibrary.PrintString` "Player interacted" true true (struct :`R` 1.0 :`G` 0.73919 :`A` 1.0))
  (bind _asbp_player_pawn (cast `/Game/Blueprints/Actors/Characters/BP_PlayerPawn` (`GameplayStatics.GetPlayerCharacter` 0)))
  (`|AddComponentByClass` _asbp_player_pawn "/Game/Blueprints/Components/C_ChildEffectComponent-DUPLICATE-THIS.C_ChildEffectComponent-DUPLICATE-THIS_C"))

(fn `UserConstructionScript`
  ;[1 1 1] Set interact range
  (`SphereComponent.SetSphereRadius` (`self.InteractRangeSphere`) (`self.InteractRange`) true))