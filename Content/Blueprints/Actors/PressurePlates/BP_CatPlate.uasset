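; BP_CatPlate is a pressure plate that responds only to the cat pawn.
; It registers itself with a Manager on BeginPlay through PlateCounter.
; When a BP_CatPawn overlaps its box collision, the plate saves its position, drops slightly without sweeping and notifies the Manager that it is activated.
; When the cat leaves, the plate returns to the saved position and reports deactivation.
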(event `self.ReceiveBeginPlay`
  (`/Game/Blueprints/Actors/PressurePlates/BP_PressurePlatePuzzleManager.PlateCounter` (`self.Manager`)))

(event `self.BoxCollision.OnComponentBeginOverlap`
  (params (OverlappedComponent :type "PrimitiveComponent Object Reference") (OtherActor :type "Actor Object Reference") (OtherComp :type "PrimitiveComponent Object Reference") (OtherBodyIndex :type Integer) (bFromSweep :type Boolean) (SweepResult :type "HitResult Structure (by ref)"))
  (bind _returnvalue (`SceneComponent.K2_GetComponentLocation` (`self.Plate`)))
  (cast `/Game/Blueprints/Actors/Characters/BP_CatPawn` OtherActor)
  (set `self.OriginalPlateLocation` _returnvalue)
  (`SceneComponent.K2_SetWorldLocation` (`self.Plate`) (- _returnvalue (0.0 0.0 10.0)) false false)
  (`/Game/Blueprints/Actors/PressurePlates/BP_PressurePlatePuzzleManager.PlateActivated` (`self.Manager`)))

(event `self.BoxCollision.OnComponentEndOverlap`
  (params (OverlappedComponent :type "PrimitiveComponent Object Reference") (OtherActor :type "Actor Object Reference") (OtherComp :type "PrimitiveComponent Object Reference") (OtherBodyIndex :type Integer))
  (cast `/Game/Blueprints/Actors/Characters/BP_CatPawn` OtherActor)
  (`SceneComponent.K2_SetWorldLocation` (`self.Plate`) (`self.OriginalPlateLocation`) false false)
  (`/Game/Blueprints/Actors/PressurePlates/BP_PressurePlatePuzzleManager.PlateDeactivated` (`self.Manager`)))

(fn `UserConstructionScript`)