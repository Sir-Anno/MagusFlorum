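; Puzzle manager Blueprint that opens a linked door when all of its pressure plates are active at once.
; A registration event increments the total plate count, while activation and deactivation events raise and lower the active count.
; When an activation makes the active count equal the total, it calls OpenDoor on the door; deactivation never closes it.
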(event `PlatesCounter`
  (`/Engine/EditorBlueprintResources/StandardMacros.IncrementInt` (`self.TotalPlates`)))

(event `PlateActivated`
  (bind _result (`/Engine/EditorBlueprintResources/StandardMacros.IncrementInt` (`self.ActivePlates`))
    (:`  `
      (if (== _result (`self.TotalPlates`))
        (`/Game/Blueprints/Actors/BP_OpenableDoor.OpenDoor` (`self.Door`))))))

(event `Plate Deactivated`
  (`/Engine/EditorBlueprintResources/StandardMacros.DecrementInt` (`self.ActivePlates`)))

(fn `UserConstructionScript`)