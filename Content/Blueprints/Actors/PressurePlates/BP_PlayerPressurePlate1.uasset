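; Player pressure plate actor for a puzzle that slides toward an offset when its box is overlapped and back when the overlap ends.
; A Movement timeline lerps the location and calls ActivatePlate on every update, where a FlipFlop toggles PlateActive.
; Puzzlestart sets a looping timer for an apparently unfinished PatternReveal, whose switch cases all apply a red mushroom material to the plate and re-set the timer.
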(event `self.ReceiveBeginPlay`
  (set `self.PlateActive` false)
  (set `self.StartLocation` (`self.K2_GetActorLocation`)))

(event `self.BoxCollision.OnComponentBeginOverlap`
  (params (OverlappedComponent :type "PrimitiveComponent Object Reference") (OtherActor :type "Actor Object Reference") (OtherComp :type "PrimitiveComponent Object Reference") (OtherBodyIndex :type Integer) (bFromSweep :type Boolean) (SweepResult :type "HitResult Structure (by ref)"))
  (bind _startlocation (`self.StartLocation`))
  (bind (_direction _alpha) (`Timeline|Movement` :!label _label)
    (:`Update`
      (`self.K2_SetActorLocation` (`KismetMathLibrary.VLerp` _startlocation (+ _startlocation (`self.TargetLocation`)) _alpha))
      (`self.ActivatePlate`))))

(event `self.BoxCollision.OnComponentEndOverlap`
  (params (OverlappedComponent :type "PrimitiveComponent Object Reference") (OtherActor :type "Actor Object Reference") (OtherComp :type "PrimitiveComponent Object Reference") (OtherBodyIndex :type Integer))
  (goto _label :!via `Reverse`))

(event `ActivatePlate`
  (`/Engine/EditorBlueprintResources/StandardMacros.FlipFlop`
    (:`A`
      (set `self.PlateActive` true))
    (:`B`
      (set `self.PlateActive` false))))

(event `Puzzle start`
  (bind _returnvalue (`KismetSystemLibrary.K2_SetTimerDelegate` (delegate `PatternReveal`) 2.0 true :!label _label_2)))

(event `PatternReveal`
  (bind _plate (`self.Plate`))
  (switch `int` (`KismetMathLibrary.FTrunc` (`KismetSystemLibrary.K2_GetTimerElapsedTimeHandle` (stale `Puzzle start` _returnvalue)))
    (:`0`
      _)
    (:`1`
      _)
    (:`2`
      _)
    (:`3`
      _)
    (:`4`
      _))
  (for (_ _array_index) (`|MakeArray` _plate)
    (`PrimitiveComponent.SetMaterial` _plate _array_index "/Game/Assets/Materials/M_MushroomRed.M_MushroomRed")
    (goto _label_2)))

(fn `UserConstructionScript`)