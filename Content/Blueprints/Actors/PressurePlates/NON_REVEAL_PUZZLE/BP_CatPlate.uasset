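; BP_CatPlate is a pressure plate for a puzzle, triggered only when a BP_CatPawn overlaps its box collision.
; It registers with a Manager on BeginPlay, then a timeline lerps it slightly downward on overlap and reverses when the overlap ends.
; When the timeline finishes in either direction, it reports activation or deactivation to the Manager based on its PlateActive flag.
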(event `self.ReceiveBeginPlay`
  (bind _manager (`self.Manager`))
  (bind _output_get (set `self.StartLocation` (`self.K2_GetActorLocation`)))
  (set `self.TargetLocation` (- _output_get (0.0 0.0 5.0)))
  (`/Engine/EditorBlueprintResources/StandardMacros.IsValid` _manager
    (:`Is Valid`
      (`/Game/Blueprints/Actors/PressurePlates/NON_REVEAL_PUZZLE/BP_PressurePlateManager.PlatesCounter` _manager))))

(event `self.BoxCollision.OnComponentBeginOverlap`
  (params (OverlappedComponent :type "PrimitiveComponent Object Reference") (OtherActor :type "Actor Object Reference") (OtherComp :type "PrimitiveComponent Object Reference") (OtherBodyIndex :type Integer) (bFromSweep :type Boolean) (SweepResult :type "HitResult Structure (by ref)"))
  (bind _manager (`self.Manager`))
  (cast `/Game/Blueprints/Actors/Characters/BP_CatPawn` OtherActor)
  (set `self.PlateActive` true)
  (bind (_direction _alpha) (`Timeline|Timeline_0` :!label _label)
    (:`Update`
      (`self.K2_SetActorLocation` (`KismetMathLibrary.VLerp` (`self.StartLocation`) (`self.TargetLocation`) _alpha)))
    (:`Finished`
      (`/Engine/EditorBlueprintResources/StandardMacros.IsValid` (`self.Manager`)
        (:`Is Valid`
          (if (`self.PlateActive`)
            (`/Game/Blueprints/Actors/PressurePlates/NON_REVEAL_PUZZLE/BP_PressurePlateManager.PlateActivated` _manager)
            (else
              (`/Game/Blueprints/Actors/PressurePlates/NON_REVEAL_PUZZLE/BP_PressurePlateManager.PlateDeactivated` _manager))))))))

(event `self.BoxCollision.OnComponentEndOverlap`
  (params (OverlappedComponent :type "PrimitiveComponent Object Reference") (OtherActor :type "Actor Object Reference") (OtherComp :type "PrimitiveComponent Object Reference") (OtherBodyIndex :type Integer))
  (cast `/Game/Blueprints/Actors/Characters/BP_CatPawn` OtherActor)
  (set `self.PlateActive` false)
  (goto _label :!via `Reverse`))

(fn `UserConstructionScript`)