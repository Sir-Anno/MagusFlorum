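; BP_PlantPlate is a pressure plate actor that registers itself with a puzzle Manager on BeginPlay.
; Its activation logic, a timeline lerping the plate 5 units down or back and then notifying the Manager of activation or deactivation, is disconnected.
; Both box overlap events are empty, so the plate never moves or reports a state change as it stands.
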(event `self.ReceiveBeginPlay`
  (bind _manager (`self.Manager`))
  (bind _output_get (set `self.StartLocation` (`self.K2_GetActorLocation`)))
  (set `self.TargetLocation` (- _output_get (0.0 0.0 5.0)))
  (`/Engine/EditorBlueprintResources/StandardMacros.IsValid` _manager
    (:`Is Valid`
      (`/Game/Blueprints/Actors/PressurePlates/NON_REVEAL_PUZZLE/BP_PressurePlateManager.PlatesCounter` _manager))))

(event `self.BoxCollision.OnComponentBeginOverlap`
  (params (OverlappedComponent :type "PrimitiveComponent Object Reference") (OtherActor :type "Actor Object Reference") (OtherComp :type "PrimitiveComponent Object Reference") (OtherBodyIndex :type Integer) (bFromSweep :type Boolean) (SweepResult :type "HitResult Structure (by ref)")))

(event `self.BoxCollision.OnComponentEndOverlap`
  (params (OverlappedComponent :type "PrimitiveComponent Object Reference") (OtherActor :type "Actor Object Reference") (OtherComp :type "PrimitiveComponent Object Reference") (OtherBodyIndex :type Integer)))

(fn `UserConstructionScript`)