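; BP_PlayerPressurePlate is a pressure plate actor that moves when its box collision is overlapped and returns when the overlap ends.
; The Movement timeline plays or reverses, lerping the actor from its start location by the TargetLocation offset.
; Every timeline update, in either direction, also calls ActivatePlate, whose FlipFlop toggles PlateActive, so the flag alternates throughout the movement rather than tracking whether the plate is pressed.
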(event `self.ReceiveBeginPlay`
  (set `self.PlateActive` false)
  (set `self.StartLocation` (`self.K2_GetActorLocation`)))

(event `self.BoxCollision.OnComponentBeginOverlap`
  (params (OverlappedComponent :type "PrimitiveComponent Object Reference") (OtherActor :type "Actor Object Reference") (OtherComp :type "PrimitiveComponent Object Reference") (OtherBodyIndex :type Integer) (bFromSweep :type Boolean) (SweepResult :type "HitResult Structure (by ref)"))
  (bind _startlocation (`self.StartLocation`))
  (bind (_direction _alpha) (`Timeline|Movement` :!label _label)
    (:`Update`
      (`self.K2_SetActorLocation` (`KismetMathLibrary.VLerp` _startlocation (+ _startlocation (`self.TargetLocation`)) _alpha))
      (`self.ActivatePlate`))))

(event `self.BoxCollision.OnComponentEndOverlap`
  (params (OverlappedComponent :type "PrimitiveComponent Object Reference") (OtherActor :type "Actor Object Reference") (OtherComp :type "PrimitiveComponent Object Reference") (OtherBodyIndex :type Integer))
  (goto _label :!via `Reverse`))

(event `ActivatePlate`
  (`/Engine/EditorBlueprintResources/StandardMacros.FlipFlop`
    (:`A`
      (set `self.PlateActive` true))
    (:`B`
      (set `self.PlateActive` false))))

(fn `UserConstructionScript`)