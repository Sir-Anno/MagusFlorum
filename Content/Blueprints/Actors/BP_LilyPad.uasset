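; Lily pad actor that moves along a spline while objects of allowed types rest on it and moves back once it is empty.
; Mesh hits add actors to a tracked list, and leaving the Box overlap removes them, updating the occupied flag.
; Tick raises or lowers a clamped 0–1 alpha at FallingSpeed, then places the mesh at that time on the LilyPadMovement spline with constant velocity.
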(event `RemoveActorFromTheLily`
  (params (actor :type "Actor Object Reference"))
  (bind _returnvalue (`KismetArrayLibrary.Array_RemoveItem` (`self.ObjectsOnTopOfIt`) actor))
  (if (and _returnvalue (== (`KismetArrayLibrary.Array_Length` (`self.ObjectsOnTopOfIt`)) 0))
    (set `self.isCharacterOnTopOfIt` false)))

(event `self.Mesh.OnComponentHit`
  (params (HitComponent :type "PrimitiveComponent Object Reference") (OtherActor :type "Actor Object Reference") (OtherComp :type "PrimitiveComponent Object Reference") (NormalImpulse :type "Vector Structure") (Hit :type "HitResult Structure (by ref)"))
  (if (`KismetArrayLibrary.Array_Contains` (`self.ActorTypesThatInteract`) (`GameplayStatics.GetObjectClass` OtherActor))
    (`KismetArrayLibrary.Array_AddUnique` (`self.ObjectsOnTopOfIt`) OtherActor)
    (set `self.isCharacterOnTopOfIt` true)))

(event `self.Box.OnComponentEndOverlap`
  (params (OverlappedComponent :type "PrimitiveComponent Object Reference") (OtherActor :type "Actor Object Reference") (OtherComp :type "PrimitiveComponent Object Reference") (OtherBodyIndex :type Integer))
  (`self.RemoveActorFromTheLily` OtherActor))

(event `self.ReceiveTick`
  (params (DeltaSeconds :type "Float (single-precision)"))
  (bind _currentalpha (`self.currentAlpha`))
  (bind _returnvalue (* DeltaSeconds (`self.FallingSpeed`)))
  (bind _returnvalue_2 (`KismetMathLibrary.SelectFloat` (+ _returnvalue _currentalpha) (- _currentalpha _returnvalue) (`self.isCharacterOnTopOfIt`)))
  (bind _returnvalue_3 (`KismetMathLibrary.SelectFloat` 0.0 _returnvalue_2 (< _returnvalue_2 0.0)))
  (bind _output_get (set `self.currentAlpha` (`KismetMathLibrary.SelectFloat` 1.0 _returnvalue_3 (> _returnvalue_3 1.0))))
  (`self.UpdateMeshPosition` _output_get))

(event `UpdateMeshPosition`
  (params (alpha :type "Float (double-precision)"))
  (`SceneComponent.K2_SetWorldLocation` (`self.Mesh`) (`SplineComponent.GetLocationAtTime` (`self.LilyPadMovement`) alpha "World" true) false false))

(fn `UserConstructionScript`)