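; BP_EndLevelTrigger is an interactable end-of-level spot where the player deposits collected kittens toward the win condition.
; On BeginPlay it sets the game mode's CatsNeeded from the number of BP_KittenPickup actors in the level.
; Each interaction moves one collected cat onto the next of six placement points as a spawned static mesh, then checks the win condition.
; A DoOnce with a short delayed reset blocks double placement.
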(event `self.ReceiveBeginPlay`
  ;[1 1 1] Init
  (bind _asgm_magus_florum (cast `/Game/Blueprints/Gamemodes/GM_MagusFlorum` (`GameplayStatics.GetGameMode`)))
  (set `self.GM ref` _asgm_magus_florum)
  (bind _outactors (`GameplayStatics.GetAllActorsOfClass` "/Game/Blueprints/Actors/Items/BP_KittenPickup.BP_KittenPickup_C"))
  (set `/Game/Blueprints/Gamemodes/GM_MagusFlorum.Cats needed` (`KismetArrayLibrary.Array_Length` _outactors) (`self.GM ref`)))

(event `/Game/Blueprints/Interfaces/BI_Interact.Interact`
  (params (Player :type "Character Object Reference"))
  ;[1 1 1] Player interaction
  (if (> (`/Game/Blueprints/Gamemodes/GM_MagusFlorum.Cats collected` (`self.GM ref`)) 0)
    (`/Engine/EditorBlueprintResources/StandardMacros.DoOnce` false :!label _label
      (:`Completed`
        (`/Engine/EditorBlueprintResources/StandardMacros.DecrementInt` (`/Game/Blueprints/Gamemodes/GM_MagusFlorum.Cats collected` (`self.GM ref`))
          (:`  `
            (`/Engine/EditorBlueprintResources/StandardMacros.DecrementInt` (`/Game/Blueprints/Gamemodes/GM_MagusFlorum.Cats needed` (`self.GM ref`))
              (:`  `
                (bind _result (`/Engine/EditorBlueprintResources/StandardMacros.IncrementInt` (`self.Cats placed`))
                  (:`  `
                    (`self.Place cat` _result)))))))))
    (else
      (`KismetSystemLibrary.PrintString` "You need to collect a cat first!" true true (struct :`R` 1.0 :`G` 0.373139 :`A` 1.0)))))

(event `Reset`
  ;[1 1 1] Player interaction
  (goto _label :!via `Reset`))

(event `Place cat`
  (params (`Cats placed` :type Integer))
  ;[1 1 1] Place cat
  (switch `int` `Cats placed`
    (:`1`
      (set `self.Cat spawn loc` (`SceneComponent.RelativeLocation` (`self.Cat place 1`))))
    (:`2`
      (set `self.Cat spawn loc` (`SceneComponent.RelativeLocation` (`self.Cat place 2`))))
    (:`3`
      (set `self.Cat spawn loc` (`SceneComponent.RelativeLocation` (`self.Cat place 3`))))
    (:`4`
      (set `self.Cat spawn loc` (`SceneComponent.RelativeLocation` (`self.Cat place 4`))))
    (:`5`
      (set `self.Cat spawn loc` (`SceneComponent.RelativeLocation` (`self.Cat place 5`))))
    (:`6`
      (set `self.Cat spawn loc` (`SceneComponent.RelativeLocation` (`self.Cat place 6`)))))
  (`AddComponent|NODE_AddStaticMeshComponent-0` :`RelativeTransform` (`KismetMathLibrary.MakeTransform` (`self.Cat spawn loc`) (struct) (0.3 0.3 0.3)))
  (`KismetSystemLibrary.PrintString` "Cat placed!" true true (struct :`R` 0.056174 :`G` 1.0 :`A` 1.0))
  (`KismetSystemLibrary.Delay` 0.2) ; Delay reset or else \nplacement triggers twice
  (`self.Reset`)
  (`/Game/Blueprints/Gamemodes/GM_MagusFlorum.Check win condition` (`self.GM ref`)))

(fn `UserConstructionScript`
  (`parent.UserConstructionScript`))