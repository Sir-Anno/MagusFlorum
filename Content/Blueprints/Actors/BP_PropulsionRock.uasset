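; A platform actor that hovers in place and launches along an offset after a player pawn stands on it for a set delay.
; A Hover timeline lerps its location, re-reading start and end from the current position each cycle.
; Overlap starts a timer that stops hovering and plays the Propell timeline from the construction-time location.
; Stepping off cancels the timer and reverses Propell; hovering restarts when Propell finishes.
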(event `self.ReceiveBeginPlay`
  ;[1 1 1] Hover animation
  (`TimelineComponent.SetPlayRate` (`self.Hover`) (`self.Hover speed`))
  (`self.Set hover vectors` :!label _label) ; Sets the locations to hover between
  (bind (_direction _alpha) (`Timeline|Hover` :!via `PlayFromStart`)
    (:`Update`
      (`self.K2_SetActorLocation` (`KismetMathLibrary.VLerp` (`self.Hover start vec`) (`self.Hover end vec`) _alpha)))
    (:`Finished`
      (`self.Restart hover`))))

(event `Restart hover`
  ;[1 1 1] Hover animation
  (goto _label))

(event `self.Collision box.OnComponentBeginOverlap`
  (params (OverlappedComponent :type "PrimitiveComponent Object Reference") (OtherActor :type "Actor Object Reference") (OtherComp :type "PrimitiveComponent Object Reference") (OtherBodyIndex :type Integer) (bFromSweep :type Boolean) (SweepResult :type "HitResult Structure (by ref)"))
  ;[1 1 1] Propulstion animation
  (cast `/Game/Blueprints/Actors/Characters/BP_PlayerPawn` OtherActor)
  (bind _returnvalue (`KismetSystemLibrary.K2_SetTimerDelegate` (delegate `Launch`) (`self.Launch delay`))) ; Wait before launching platform
  (set `self.Launch delay timer ref` _returnvalue))

(event `Launch`
  (bind _propell_start_vec (`self.Propell start vec`))
  ;[1 1 1] Propulstion animation
  ;;[1 1 1] Stop the hovering animation before moving
  (`TimelineComponent.Stop` (`self.Hover`))
  (bind (_direction _alpha) (`Timeline|Propell` :!via `PlayFromStart` :!label _label_2)
    (:`Update`
      (`self.K2_SetActorLocation` (`KismetMathLibrary.VLerp` _propell_start_vec (+ _propell_start_vec (`self.Propell end vec`)) _alpha)))
    (:`Finished`
      (`TimelineComponent.Stop` (`self.Propell`))
      (`self.Restart hover`))))

(event `self.Collision box.OnComponentEndOverlap`
  (params (OverlappedComponent :type "PrimitiveComponent Object Reference") (OtherActor :type "Actor Object Reference") (OtherComp :type "PrimitiveComponent Object Reference") (OtherBodyIndex :type Integer))
  ;[1 1 1] Propulstion animation
  (cast `/Game/Blueprints/Actors/Characters/BP_PlayerPawn` OtherActor)
  (`KismetSystemLibrary.K2_ClearAndInvalidateTimerHandle` (`self.Launch delay timer ref`)) ; If player leaves platform before launch cancel launch
  ;;[1 1 1] Stop the hovering animation before moving
  (`TimelineComponent.Stop` (`self.Hover`))
  (goto _label_2 :!via `Reverse`))

(fn `Set hover vectors`
  (bind _output_get (set `self.Hover start vec` (`self.K2_GetActorLocation`)))
  (set `self.Hover end vec` (+ _output_get (`self.Hover offset`))))

(fn `UserConstructionScript`
  (set `self.Propell start vec` (`self.K2_GetActorLocation`)))