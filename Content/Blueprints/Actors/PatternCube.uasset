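; PatternCube is an interactable cube actor that displays four text labels and rotates when interacted with.
; BeginPlay caches its starting transform and fills labels A to D from text values.
; Interact replays a timeline from the start, lerping rotation between the start rotation combined with TargetRotation (alpha 0) and the start rotation (alpha 1).
; Rotations do not accumulate across interactions, and the cached location is unused.
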(event `self.ReceiveBeginPlay`
  (set `self.StartLocation` (`self.K2_GetActorLocation`))
  (set `self.StartRotation` (`self.K2_GetActorRotation`))
  (`TextRenderComponent.K2_SetText` (`self.A`) (`self.Value`))
  (`TextRenderComponent.K2_SetText` (`self.B`) (`self.Value_0`))
  (`TextRenderComponent.K2_SetText` (`self.C`) (`self.Value_1`))
  (`TextRenderComponent.K2_SetText` (`self.D`) (`self.Value_2`)))

(event `/Game/Blueprints/Interfaces/BI_Interact.Interact`
  (params (Player :type "/Game/Blueprints/Actors/Characters/BP_PlayerPawn Object Reference"))
  (bind _startrotation (`self.StartRotation`))
  (bind (_direction _alpha) (`Timeline|RotationTimeline` :!via `PlayFromStart`)
    (:`Update`
      (`self.K2_SetActorRotation` (`KismetMathLibrary.RLerp` (`KismetMathLibrary.ComposeRotators` _startrotation (`self.TargetRotation`)) _startrotation _alpha)))))

(fn `UserConstructionScript`)