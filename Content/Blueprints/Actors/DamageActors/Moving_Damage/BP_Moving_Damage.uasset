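; BP_Moving_Damage is a moving hazard actor that damages the player on contact.
; On BeginPlay, the Moving timeline drives the Cube's relative location without sweep.
; A 3-second Delay off the timeline's Update toggles IsLooped, alternating Play and Reverse to keep it moving back and forth.
; When BP_PlayerPawn overlaps the Box, the actor applies Damage through the pawn's CHealthComponent.
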(event `self.ReceiveBeginPlay`
  ;[1 1 1] Actor Moves according to the timeline
  (bind (_direction _moving) (`Timeline|Moving` :!label _label) ; Spped and how far it moves are in here
    (:`Update`
      (`SceneComponent.K2_SetRelativeLocation` (`self.Cube`) _moving false false) ; How it moves
      (`KismetSystemLibrary.Delay` 3.0)
      (if (`self.IsLooped`)
        (set `self.IsLooped` false)
        (goto _label :!via `Reverse`)
        (else
          (set `self.IsLooped` true)
          (goto _label))))))

(event `self.Box.OnComponentBeginOverlap`
  (params (OverlappedComponent :type "PrimitiveComponent Object Reference") (OtherActor :type "Actor Object Reference") (OtherComp :type "PrimitiveComponent Object Reference") (OtherBodyIndex :type Integer) (bFromSweep :type Boolean) (SweepResult :type "HitResult Structure (by ref)"))
  ;[1 0.003447 0] To Damage
  (bind _asbp_player_pawn (cast `/Game/Blueprints/Actors/Characters/BP_PlayerPawn` OtherActor))
  (`/Game/Blueprints/Components/C_HealthComponent.Take damage` (`/Game/Blueprints/Actors/Characters/BP_PlayerPawn.C_HealthComponent` _asbp_player_pawn) (`self.Damage`)) ; Takes the damage away
)

(fn `UserConstructionScript`)