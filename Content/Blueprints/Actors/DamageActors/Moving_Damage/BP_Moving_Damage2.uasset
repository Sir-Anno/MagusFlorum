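; BP_Moving_Damage2 is a moving hazard actor that damages the player on contact.
; The construction script sets InterpToMovement to travel between two relative locations over a configurable duration.
; When its Box overlaps a BP_PlayerPawn, it calls TakeDamage on that pawn's health component with its Damage value.
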(event `self.Box.OnComponentBeginOverlap`
  (params (OverlappedComponent :type "PrimitiveComponent Object Reference") (OtherActor :type "Actor Object Reference") (OtherComp :type "PrimitiveComponent Object Reference") (OtherBodyIndex :type Integer) (bFromSweep :type Boolean) (SweepResult :type "HitResult Structure (by ref)"))
  ;[1 0.03242 0] Damage
  (bind _asbp_player_pawn (cast `/Game/Blueprints/Actors/Characters/BP_PlayerPawn` OtherActor))
  (`/Game/Blueprints/Components/C_HealthComponent.Take damage` (`/Game/Blueprints/Actors/Characters/BP_PlayerPawn.C_HealthComponent` _asbp_player_pawn) (`self.Damage`)) ; Takes the damage away
)

(fn `UserConstructionScript`
  (bind _interptomovement (`self.InterpToMovement`))
  (set `InterpToMovementComponent.ControlPoints` (`|MakeArray` (make `InterpControlPoint` (`self.Location_1`)) (make `InterpControlPoint` (`self.Location_2`))) _interptomovement)
  (set `InterpToMovementComponent.Duration` (`self.Duration`) _interptomovement))