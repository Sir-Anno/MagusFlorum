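; BP_Spore is a mushroom hazard that releases a damaging spore cloud when something comes near or lands on its cap.
; The proximity sphere and top collision each play build-up animations, wait, then spawn particles and a BP_SporeAttack actor.
; Proximity attacks use a configurable position and scale, while cap attacks use the actor's location.
; Leaving destroys the stored attack after a delay; every handler has an unreset DoOnce, so each runs once.
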(event `self.Sphere.OnComponentBeginOverlap`
  (params (OverlappedComponent :type "PrimitiveComponent Object Reference") (OtherActor :type "Actor Object Reference") (OtherComp :type "PrimitiveComponent Object Reference") (OtherBodyIndex :type Integer) (bFromSweep :type Boolean) (SweepResult :type "HitResult Structure (by ref)"))
  (bind _sporeattackscale (`self.SporeAttackScale`))
  (bind _returnvalue (`SceneComponent.K2_GetComponentLocation` (`self.SporeAttackPosition`)))
  ;[1 1 1] Spore Attacks you if near
  (`/Engine/EditorBlueprintResources/StandardMacros.DoOnce` false ; It will create an infinite loops of trying to kill you unless you have this
    (:`Completed`
      (`SkeletalMeshComponent.PlayAnimation` (`self.Mushroom`) "/Game/Assets/Animations/Mushroom/Mushrooms_Animations/BuildUpandRelase.BuildUpandRelase" false)
      (`KismetSystemLibrary.Delay` 3.0)
      (`NiagaraFunctionLibrary.SpawnSystemAtLocation` "/Game/Blueprints/Actors/DamageActors/Spores/Temp.Temp" _returnvalue (struct) (/ _sporeattackscale (5.0 5.0 10.0))) ; Spawns in particles for the spores
      (bind _returnvalue_2 (`|SpawnActorFromClass` "/Game/Blueprints/Actors/DamageActors/Spores/BP_SporeAttack.BP_SporeAttack_C" (`KismetMathLibrary.MakeTransform` _returnvalue (struct) _sporeattackscale) "Undefined" "OverrideRootScale" null null)) ; Spawns in the damage area for the spore
      (bind _output_get (set `self.AttackSpore` _returnvalue_2)))))

(event `self.Sphere.OnComponentEndOverlap`
  (params (OverlappedComponent :type "PrimitiveComponent Object Reference") (OtherActor :type "Actor Object Reference") (OtherComp :type "PrimitiveComponent Object Reference") (OtherBodyIndex :type Integer))
  ;[1 1 1] Spore Attacks you if near
  (`KismetSystemLibrary.Delay` 5.0)
  (`/Engine/EditorBlueprintResources/StandardMacros.DoOnce` false ; It will create an infinite loops of trying to kill you unless you have this
    (:`Completed`
      (`self.K2_DestroyActor` (`self.AttackSpore`))
      (`self.K2_DestroyActor` (stale `self.Sphere.OnComponentBeginOverlap` _output_get)) ; So you can walk away from it
      (`SkeletalMeshComponent.PlayAnimation` (`self.Mushroom`) "/Game/Assets/Animations/Mushroom/Mushroom_Anim_MushroomArmature_ReturnToNormal.Mushroom_Anim_MushroomArmature_ReturnToNormal" false))))

(event `self.MushroomTopCollision.OnComponentBeginOverlap`
  (params (OverlappedComponent :type "PrimitiveComponent Object Reference") (OtherActor :type "Actor Object Reference") (OtherComp :type "PrimitiveComponent Object Reference") (OtherBodyIndex :type Integer) (bFromSweep :type Boolean) (SweepResult :type "HitResult Structure (by ref)"))
  (bind _returnvalue (`self.K2_GetActorLocation`))
  (bind _mushroom (`self.Mushroom`))
  ;[1 1 1] Jumping On the Mushroom
  (`/Engine/EditorBlueprintResources/StandardMacros.DoOnce` false ; It will create an infinite loops of trying to kill you unless you have this
    (:`Completed`
      (`SkeletalMeshComponent.PlayAnimation` _mushroom "/Game/Assets/Animations/Mushroom/Mushroom_Anim_MushroomArmature_OnJump.Mushroom_Anim_MushroomArmature_OnJump" false)
      (`KismetSystemLibrary.Delay` 0.2)
      (`SkeletalMeshComponent.PlayAnimation` _mushroom "/Game/Assets/Animations/Mushroom/Mushrooms_Animations/BuildUpandRelase.BuildUpandRelase" false)
      (`KismetSystemLibrary.Delay` 3.0)
      (`NiagaraFunctionLibrary.SpawnSystemAtLocation` "/Game/Blueprints/Actors/DamageActors/Spores/Temp.Temp" _returnvalue) ; Spawns in particles for the spores
      (bind _returnvalue_2 (`|SpawnActorFromClass` "/Game/Blueprints/Actors/DamageActors/Spores/BP_SporeAttack.BP_SporeAttack_C" (`KismetMathLibrary.MakeTransform` _returnvalue (struct) (5.0 5.0 10.0)) "Undefined" "OverrideRootScale" null null)) ; Spawns in the damage area for the spore
      (bind _output_get (set `self.AttackSpore` _returnvalue_2)))))

(event `self.MushroomTopCollision.OnComponentEndOverlap`
  (params (OverlappedComponent :type "PrimitiveComponent Object Reference") (OtherActor :type "Actor Object Reference") (OtherComp :type "PrimitiveComponent Object Reference") (OtherBodyIndex :type Integer))
  ;[1 1 1] Jumping On the Mushroom
  (`KismetSystemLibrary.Delay` 5.0)
  (`/Engine/EditorBlueprintResources/StandardMacros.DoOnce` false ; It will create an infinite loops of trying to kill you unless you have this
    (:`Completed`
      (`self.K2_DestroyActor` (`self.AttackSpore`))
      (`self.K2_DestroyActor` (stale `self.MushroomTopCollision.OnComponentBeginOverlap` _output_get)) ; So you can walk away from it
      (`SkeletalMeshComponent.PlayAnimation` (`self.Mushroom`) "/Game/Assets/Animations/Mushroom/Mushroom_Anim_MushroomArmature_ReturnToNormal.Mushroom_Anim_MushroomArmature_ReturnToNormal" false))))

(fn `UserConstructionScript`)