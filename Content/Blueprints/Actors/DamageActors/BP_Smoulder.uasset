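; BP_Smoulder is an enemy character that wanders random navmesh points and attacks characters it sees through PawnSensing.
; On sight it plays an angry montage, swaps its eye material, jumps, then AI-moves to the target's location sampled after the jump.
; On arrival it applies damage in three distance tiers.
; After a hit or failed move it calms down and resumes patrol, but a target beyond the far radius leaves it in chase state.
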(event `self.ReceiveBeginPlay`
  (`self.UpdateMaterials`)
  (if (`self.shouldPatrolOnStart`)
    (`self.GoToRandomCloseLoaction`)))

(event `self.PawnSensing.OnSeePawn`
  (params (Pawn :type "Pawn Object Reference"))
  ;[1 1 1] Moves the actor to player (REQUIRES NAVMESH)
  (if (not (`self.isChasingPlayer`))
    (bind _ascharacter (cast `Character` Pawn))
    (if (!= _ascharacter self)
      (set `self.As Character` _ascharacter)
      (set `self.isChasingPlayer` true)
      (`self.Attack`))))

(event `UpdateMaterials`
  ;[1 1 1] UpdateMaterials
  (`PrimitiveComponent.SetMaterial` (`self.Mesh`) 1 (select `bool` (`self.isChasingPlayer`) :`false` (`self.PeacfulEyesMaterial`) :`true` (`self.AngryEyesMaterial`) :!type "MaterialInterface Object Reference")))

(event `GoToRandomCloseLoaction`
  ;[1 1 1] Moves the actor to player (REQUIRES NAVMESH)
  (`KismetSystemLibrary.Delay` (`self.WaitBeforeEachPatrol`))
  (`|AIMoveTo` self (`NavigationSystemV1.K2_GetRandomLocationInNavigableRadius` (`KismetMathLibrary.Conv_DoubleToVector` (`SkeletalMeshComponent.GetPosition` (`self.Mesh`))) (`self.PatrolRadiusFromPosition`) null null) null
    (:`OnSuccess`
      _)
    (:`OnFail`
      _))
  (if (not (`self.isChasingPlayer`))
    (`self.GoToRandomCloseLoaction`)))

(event `Attack`
  (bind _as_character (`self.As Character`))
  (`|PlayMontage` (`self.Mesh`) "/Game/Assets/Meshes/Oldin_Soukup/Smoulder_Anim_BeAngry_Montage.Smoulder_Anim_BeAngry_Montage"
    (:`then`
      (`self.UpdateMaterials`)
      (`KismetSystemLibrary.Delay` (`self.PreJumpDelay`))
      (`self.Jump`)
      (`KismetSystemLibrary.Delay` (`self.MidAirDelay`))
      (`/Engine/EditorBlueprintResources/StandardMacros.IsValid` _as_character
        (:`Is Valid`
          (`|AIMoveTo` self (`self.K2_GetActorLocation` _as_character) null 30.0
            (:`OnSuccess`
              (`self.DealDamage`))
            (:`OnFail`
              (`self.GoToIdle`))))))))

(event `DealDamage`
  (bind _as_character (`self.As Character`))
  (bind _as_character_2 (`self.As Character`))
  (bind _returnvalue (`KismetMathLibrary.Vector_Distance` (`self.K2_GetActorLocation` _as_character_2) (`self.K2_GetActorLocation`)))
  (`/Engine/EditorBlueprintResources/StandardMacros.IsValid` _as_character_2
    (:`Is Valid`
      (if (< _returnvalue (`self.Close range radius`))
        (`GameplayStatics.ApplyDamage` _as_character (`self.High Damage`))
        (`self.GoToIdle`)
        (elif (< _returnvalue (`self.Med range radius`))
          (`GameplayStatics.ApplyDamage` _as_character (`self.Middle Damage`))
          (`self.GoToIdle`)
          (elif (< _returnvalue (`self.Far range radius`))
            (`GameplayStatics.ApplyDamage` _as_character (`self.Low Damage`))
            (`self.GoToIdle`)))))))

(event `GoToIdle`
  (`|PlayMontage` (`self.Mesh`) "/Game/Assets/Meshes/Oldin_Soukup/Smoulder_Anim_BePeacful_Montage.Smoulder_Anim_BePeacful_Montage"
    (:`then`
      (`KismetSystemLibrary.Delay` (`self.delayBeforePatroling`))
      (set `self.isChasingPlayer` false)
      (`self.UpdateMaterials`)
      (`self.GoToRandomCloseLoaction`))))

(fn `UserConstructionScript`)