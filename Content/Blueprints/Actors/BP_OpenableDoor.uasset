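; BP_OpenableDoor is a door actor that slides open when its OpenDoor event is called.
; On BeginPlay it stores its start location and adds it to EndLocation, turning that relative offset into a world-space target.
; OpenDoor plays the T_OpenDoor timeline, whose track drives a vector lerp that moves the whole actor between the two locations without sweep.
; The Blueprint contains no closing logic.
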(event `self.ReceiveBeginPlay`
  (bind _output_get (set `self.StartLocation` (`self.K2_GetActorLocation`)))
  (set `self.EndLocation` (+ _output_get (`self.EndLocation`))))

(event `OpenDoor`
  (bind (_direction _opendoor) (`Timeline|T_OpenDoor`)
    (:`Update`
      (`self.K2_SetActorLocation` (`KismetMathLibrary.VLerp` (`self.StartLocation`) (`self.EndLocation`) _opendoor)))))

(fn `UserConstructionScript`)