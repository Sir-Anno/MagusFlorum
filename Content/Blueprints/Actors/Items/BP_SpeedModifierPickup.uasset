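; BP_SpeedModifierPickup is a pickup that applies a speed modifier effect to the player.
; It triggers either on player interaction or when a player pawn overlaps its collision sphere.
; Both paths add a C_SpeedModifierEffect component to the player with the configured multiplier and attach it to that player.
; On BeginPlay it copies its Duration into EffectDuration, overriding the base effect's value.
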(event `self.ReceiveBeginPlay`
  (set `self.EffectDuration` (`self.Duration`)) ; Over write durration in base effect
)

(event `/Game/Blueprints/Interfaces/BI_Interact.Interact`
  (params (Player :type "/Game/Blueprints/Actors/Characters/BP_PlayerPawn Object Reference"))
  (`parent.Interact` Player)
  (set `self.Player Ref` Player)
  (bind _returnvalue (`|AddComponentByClass` (`self.Player Ref`) "/Game/Blueprints/Components/C_SpeedModifierEffect.C_SpeedModifierEffect_C" (`self.Speed Multiplier`) :!label _label))
  (set `/Game/Blueprints/Components/C_BaseBuffDebuffComponent.Set attached actor` (`self.Player Ref`) _returnvalue))

(event `self.SphereCollision.OnComponentBeginOverlap`
  (params (OverlappedComponent :type "PrimitiveComponent Object Reference") (OtherActor :type "Actor Object Reference") (OtherComp :type "PrimitiveComponent Object Reference") (OtherBodyIndex :type Integer) (bFromSweep :type Boolean) (SweepResult :type "HitResult Structure (by ref)"))
  (bind _asbp_player_pawn (cast `/Game/Blueprints/Actors/Characters/BP_PlayerPawn` OtherActor))
  (set `self.Player Ref` _asbp_player_pawn)
  (goto _label))

(fn `UserConstructionScript`
  (`parent.UserConstructionScript`))