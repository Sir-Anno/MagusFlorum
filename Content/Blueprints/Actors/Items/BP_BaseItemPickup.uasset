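; BP_BaseItemPickup is a base actor for item pickups that either respawn or are destroyed when the player interacts.
; Interact hides the root and its children, waits RespawnDelay and shows them again when ShouldRespawn is set, otherwise it destroys the actor.
; Respawning toggles only visibility, leaving collision untouched.
; PlaySound plays the Audio component if valid, and the SphereCollision begin-overlap event is empty.
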(event `/Game/Blueprints/Interfaces/BI_Interact.Interact`
  (params (Player :type "Character Object Reference"))
  (if (`self.Should respawn?`)
    (`SceneComponent.SetVisibility` (`self.DefaultSceneRoot`) false true)
    (`KismetSystemLibrary.Delay` (`self.Respawn delay`))
    (`SceneComponent.SetVisibility` (`self.DefaultSceneRoot`) true true)
    (else
      (`self.K2_DestroyActor`))))

(event `PlaySound`
  (bind _audio (`self.Audio`))
  (`/Engine/EditorBlueprintResources/StandardMacros.IsValid` _audio
    (:`Is Valid`
      (`AudioComponent.Play` _audio 0.0))))

(event `self.SphereCollision.OnComponentBeginOverlap`
  (params (OverlappedComponent :type "PrimitiveComponent Object Reference") (OtherActor :type "Actor Object Reference") (OtherComp :type "PrimitiveComponent Object Reference") (OtherBodyIndex :type Integer) (bFromSweep :type Boolean) (SweepResult :type "HitResult Structure (by ref)")))

(fn `UserConstructionScript`)