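; BP_KittenPickup is a kitten item that counts toward the game stats when collected by the player or cat pawn.
; Collection fires from either the inherited Interact event or an overlap with its collision sphere.
; Both paths check for BP_PlayerPawn or BP_CatPawn, update a stat through GM_MagusFlorum, then destroy the actor.
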(event `/Game/Blueprints/Interfaces/BI_Interact.Interact`
  (params (Player :type "Character Object Reference"))
  (bind _player_ref (`self.Player ref`))
  (`parent.Interact` Player)
  (set `self.Player ref` Player)
  (`|ExecutionSequence` :!label _label
    (:`then_0`
      (cast `/Game/Blueprints/Actors/Characters/BP_PlayerPawn` _player_ref))
    (:`then_1`
      (cast `/Game/Blueprints/Actors/Characters/BP_CatPawn` _player_ref)))
  (bind _asgm_magus_florum (cast `/Game/Blueprints/Gamemodes/GM_MagusFlorum` (`GameplayStatics.GetGameMode`)))
  (`/Game/Blueprints/Gamemodes/GM_MagusFlorum.Update game stats` _asgm_magus_florum "NewEnumerator1")
  (`self.K2_DestroyActor`))

(event `self.SphereCollision.OnComponentBeginOverlap`
  (params (OverlappedComponent :type "PrimitiveComponent Object Reference") (OtherActor :type "Actor Object Reference") (OtherComp :type "PrimitiveComponent Object Reference") (OtherBodyIndex :type Integer) (bFromSweep :type Boolean) (SweepResult :type "HitResult Structure (by ref)"))
  (set `self.Player ref` OtherActor)
  (goto _label))

(fn `UserConstructionScript`
  (`parent.UserConstructionScript`))