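; BP_PuzzleKey is a key pickup that opens its assigned door when the cat pawn walks into it.
; Sphere overlap stores the overlapping actor, casts it to BP_CatPawn, then plays a sound, calls OpenDoor on DoorToUnlock and destroys the key.
; The Interact event is overridden with no action, leaving overlap as the only live trigger.
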(event `/Game/Blueprints/Interfaces/BI_Interact.Interact`
  (params (Player :type "Character Object Reference")))

(event `self.SphereCollision.OnComponentBeginOverlap`
  (params (OverlappedComponent :type "PrimitiveComponent Object Reference") (OtherActor :type "Actor Object Reference") (OtherComp :type "PrimitiveComponent Object Reference") (OtherBodyIndex :type Integer) (bFromSweep :type Boolean) (SweepResult :type "HitResult Structure (by ref)"))
  (set `self.Player ref` OtherActor)
  (cast `/Game/Blueprints/Actors/Characters/BP_CatPawn` (`self.Player ref`))
  (`self.PlaySound`)
  (`/Game/Blueprints/Actors/BP_OpenableDoor.OpenDoor` (`self.Door to unlock`))
  (`self.K2_DestroyActor`))

(fn `UserConstructionScript`
  (`parent.UserConstructionScript`))