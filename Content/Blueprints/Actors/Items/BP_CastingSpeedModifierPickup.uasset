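; Pickup that grants the player a casting speed modifier, triggered either by interacting with it or walking into its collision sphere.
; Both paths cast to BP_PlayerPawn, add a C_CastingSpeedModifier component with the configured multiplier, set the pawn as its attached actor, then destroy the pickup.
; On BeginPlay it overrides the base pickup's EffectDuration with its own Duration, though that value is not passed to the component here.
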(event `self.ReceiveBeginPlay`
  (set `self.EffectDuration` (`self.Duration`)) ; Over write durration in base pickup
)

(event `/Game/Blueprints/Interfaces/BI_Interact.Interact`
  (params (Player :type "Character Object Reference"))
  (`parent.Interact` Player)
  (bind _asbp_player_pawn (cast `/Game/Blueprints/Actors/Characters/BP_PlayerPawn` Player))
  (set `self.Player ref` _asbp_player_pawn)
  (bind _returnvalue (`|AddComponentByClass` (`self.Player ref`) "/Game/Blueprints/Components/C_CastingSpeedModifier.C_CastingSpeedModifier_C" (`self.Casting speed modifier`) :!label _label))
  (set `/Game/Blueprints/Components/C_BaseBuffDebuffComponent.Attached actor` (`self.Player ref`) _returnvalue)
  (`self.K2_DestroyActor`))

(event `self.SphereCollision.OnComponentBeginOverlap`
  (params (OverlappedComponent :type "PrimitiveComponent Object Reference") (OtherActor :type "Actor Object Reference") (OtherComp :type "PrimitiveComponent Object Reference") (OtherBodyIndex :type Integer) (bFromSweep :type Boolean) (SweepResult :type "HitResult Structure (by ref)"))
  (bind _asbp_player_pawn (cast `/Game/Blueprints/Actors/Characters/BP_PlayerPawn` OtherActor))
  (set `self.Player ref` _asbp_player_pawn)
  (goto _label))

(fn `UserConstructionScript`
  (`parent.UserConstructionScript`))