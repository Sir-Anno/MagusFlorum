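; BP_CastingSpeed is an item actor that grants a casting speed component to the actor that picks it up.
; Both player interaction and sphere overlap add a C_CastingSpeed component to that actor and copy the item's CastingSpeed value into it.
; Both paths then run the parent Interact logic and destroy the item.
; The overlap path applies to any overlapping actor, with no type check.
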(event `/Game/Blueprints/Interfaces/BI_Interact.Interact`
  (params (Player :type "/Game/Blueprints/Actors/Characters/BP_PlayerPawn Object Reference"))
  (bind _returnvalue (`|AddComponentByClass` Player "/Game/Blueprints/Components/C_CastingSpeed.C_CastingSpeed_C"))
  (set `/Game/Blueprints/Components/C_CastingSpeed.Casting Speed` (`self.Casting Speed`) _returnvalue)
  (`parent.Interact` null :!label _label)
  (`self.K2_DestroyActor`))

(event `self.SphereCollision.OnComponentBeginOverlap`
  (params (OverlappedComponent :type "PrimitiveComponent Object Reference") (OtherActor :type "Actor Object Reference") (OtherComp :type "PrimitiveComponent Object Reference") (OtherBodyIndex :type Integer) (bFromSweep :type Boolean) (SweepResult :type "HitResult Structure (by ref)"))
  (bind _returnvalue (`|AddComponentByClass` OtherActor "/Game/Blueprints/Components/C_CastingSpeed.C_CastingSpeed_C"))
  (set `/Game/Blueprints/Components/C_CastingSpeed.Casting Speed` (`self.Casting Speed`) _returnvalue)
  (goto _label))

(fn `UserConstructionScript`
  (`parent.UserConstructionScript`))