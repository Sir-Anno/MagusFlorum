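; Game Instance Blueprint that handles level progression and holds the game's SFX and music volume settings.
; Loadnextlevel opens the current LevelsList entry, then increments the index, resetting it to zero once it equals the last index.
; SetVolume stores both volumes and broadcasts them through the EDVolumeChange dispatcher.
; It also applies SFX volume directly to an AudioComponent on each actor tagged MakesSound.
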(event `Load next level`
  ;[1 1 1] Load level
  (`GameplayStatics.OpenLevelBySoftObjectPtr` (`|GetArrayItem` (`self.Levels list`) (`self.Level index`)))
  ;[1 1 1] Reset levels list index
  (`/Engine/EditorBlueprintResources/StandardMacros.IncrementInt` (`self.Level index`)
    (:`  `
      (if (== (`self.Level index`) (`KismetArrayLibrary.Array_LastIndex` (`self.Levels list`)))
        (set `self.Level index` 0)))))

(event `SetVolume`
  (params (`New SFX volume` :type "Float (double-precision)") (`New music volume` :type "Float (double-precision)"))
  ;[1 1 1] Set SFX volume on all actors in game
  (set `self.SFX volume` `New SFX volume`)
  (set `self.Music volume` `New music volume`)
  (`self.ED_VolumeChange` (`self.SFX volume`) (`self.Music volume`))
  (bind _outactors (`GameplayStatics.GetAllActorsWithTag` "MakesSound"))
  (for _array_element _outactors
    (`AudioComponent.SetVolumeMultiplier` (`Actor.GetComponentByClass` _array_element "/Script/Engine.AudioComponent") (`self.SFX volume`))))